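; BP_Lane spawns one lane section of a road-crossing style map on BeginPlay, choosing grass, highway, river or railroad from its Lane value.
; It places sections along X from SpawnerLocation, advancing CurX by a fixed step.
; Grass receives the Alternate flag as its Type.
; Highway spawns as three consecutive strips, the first with Type false and the next two true, each advancing the offset.
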(event EventBeginPlay
  (bind _spawnerlocation (Variables|Default|GetspawnerLocation))
  (bind _spawnerlocation_2 (Variables|Default|GetspawnerLocation))
  (bind _spawnerlocation_3 (Variables|Default|GetspawnerLocation))
  (Variables|Default|SetCords (Math|Vector|MakeVector (+ (Variables|Default|GetcurX) (.x _spawnerlocation)) (.y _spawnerlocation) (.z _spawnerlocation)))
  (Variables|Default|SetcurX (+ 1e+02 (Variables|Default|GetcurX)))
  (switch int (Variables|Default|Getlane)
    (:0
      (Game|SpawnActorfromClass "/Game/Map/Grass.Grass_C" (Math|Transform|MakeTransform (Variables|Default|GetCords) "0, 0, 0" "1.000000,1.000000,1.000000") "Undefined" "MultiplyWithRoot" 0 (Variables|Default|Getalternate) 0))
    (:1
      (Game|SpawnActorfromClass "/Game/Map/Highway.Highway_C" (Math|Transform|MakeTransform (Variables|Default|GetCords) "0, 0, 0" "1.000000,1.000000,1.000000") "Undefined" "MultiplyWithRoot" 0 false 0)
      (Game|SpawnActorfromClass "/Game/Map/Highway.Highway_C" (Math|Transform|MakeTransform (Math|Vector|MakeVector (+ (Variables|Default|GetcurX) (.x _spawnerlocation_2)) (.y _spawnerlocation_2) (.z _spawnerlocation_2)) "0, 0, 0" "1.000000,1.000000,1.000000") "Undefined" "MultiplyWithRoot" 0 true 0)
      (bind _output_get (Variables|Default|SetcurX (+ 1e+02 (Variables|Default|GetcurX))))
      (Game|SpawnActorfromClass "/Game/Map/Highway.Highway_C" (Math|Transform|MakeTransform (Math|Vector|MakeVector (+ _output_get (.x _spawnerlocation_3)) (.y _spawnerlocation_3) (.z _spawnerlocation_3)) "0, 0, 0" "1.000000,1.000000,1.000000") "Undefined" "MultiplyWithRoot" 0 true 0)
      (Variables|Default|SetcurX (+ 1e+02 (Variables|Default|GetcurX))))
    (:2
      (Game|SpawnActorfromClass "/Game/Map/River.River_C" (Math|Transform|MakeTransform (Variables|Default|GetCords) "0, 0, 0" "1.000000,1.000000,1.000000") "Undefined" "MultiplyWithRoot" 0 0))
    (:3
      (Game|SpawnActorfromClass "/Game/Map/Railroad.Railroad_C" (Math|Transform|MakeTransform (Variables|Default|GetCords) "0, 0, 0" "1.000000,1.000000,1.000000") "Undefined" "MultiplyWithRoot" 0 0))))

(fn ConstructionScript)