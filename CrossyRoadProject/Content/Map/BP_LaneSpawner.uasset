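; Procedural map spawner that builds endless strips of lanes along X as the player advances.
; The first spawner places a start wall and grass strips with alternating types, then a loop spawns randomly typed BP_Lane actors, each passing back the running X offset.
; A Render trigger at the segment's midpoint spawns the next BP_LaneSpawner at the segment's end, once, when the third-person character overlaps it, skipping the start area.
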(event Custom|CustomEvent
  (params (OverlappedActor :type Actor%20Object%20Reference) (OtherActor :type Actor%20Object%20Reference))
  (bind _spawnerlocation (Variables|Default|GetspawnerLocation))
  (Utilities|Casting|CastToBP_ThirdPersonCharacter OtherActor)
  (Utilities|FlowControl|DoOnce false
    (:Completed
      (Game|SpawnActorfromClass "BP_LaneSpawner_C" (Math|Transform|MakeTransform (Math|Vector|MakeVector (+ (Variables|Default|GetcurX) (.x _spawnerlocation)) (.y _spawnerlocation) (.z _spawnerlocation)) "0, 0, 0" "1.000000,1.000000,1.000000") "Undefined" "MultiplyWithRoot" 0 false 0))))

(event EventBeginPlay
  (Variables|Default|SetspawnerLocation (Transformation|GetWorldLocation (Variables|Default|GetStaticMesh)))
  (for _index (range 0 40)
    (if (Variables|Default|Getspawn)
      (Game|SpawnActorfromClass "/Game/Map/spawnWall.spawnWall_C" (Math|Transform|MakeTransform (Transformation|GetWorldLocation (Variables|Default|GetStaticMesh)) "0, 0, 0" "1.000000,1.000000,1.000000") "Undefined" "MultiplyWithRoot" 0 0)
      (Variables|Default|SetcurX (+ 1e+02 (Variables|Default|GetcurX)))
      (for _index_2 (range 0 6)
        (Game|SpawnActorfromClass "/Game/Map/Grass.Grass_C" (Math|Transform|MakeTransform (Math|Vector|MakeVector (+ (Variables|Default|GetcurX) (.x (Variables|Default|GetspawnerLocation))) (.y (Variables|Default|GetspawnerLocation)) (.z (Variables|Default|GetspawnerLocation))) "0, 0, 0" "1.000000,1.000000,1.000000") "Undefined" "MultiplyWithRoot" 0 (Variables|Default|Getalternate) 0)
        (Variables|Default|SetcurX (+ 1e+02 (Variables|Default|GetcurX)))
        (Variables|Default|Setalternate (Math|Conversions|ToInteger(Boolean) (== (Variables|Default|Getalternate) 0))))
      (Variables|Default|Setspawn false)
      (else
        (Variables|Default|Setalternate (Math|Conversions|ToInteger(Boolean) (== (Variables|Default|Getalternate) 0)))
        (bind _returnvalue (Game|SpawnActorfromClass "/Game/Map/BP_Lane.BP_Lane_C" (Math|Transform|MakeTransform "0, 0, 0" "0, 0, 0" "1.000000,1.000000,1.000000") "Undefined" "MultiplyWithRoot" 0 (Math|Random|RandomIntegerinRange 0 3) (Variables|Default|Getalternate) (Variables|Default|GetcurX) (Variables|Default|GetspawnerLocation) 0))
        (Variables|Default|SetcurX (Variables|/Game/Map/BP_Lane.BP_Lane_C|GetcurX _returnvalue)))))
  (bind _returnvalue_2 (Game|SpawnActorfromClass "/Game/Map/Render.Render_C" (Math|Transform|MakeTransform (Math|Vector|MakeVector (+ (/ (Variables|Default|GetcurX) 2.0) (.x (Variables|Default|GetspawnerLocation))) (.y (Variables|Default|GetspawnerLocation)) (.z (Variables|Default|GetspawnerLocation))) "0, 0, 0" "1.000000,1.000000,1.000000") "Undefined" "MultiplyWithRoot" 0 0))
  (EventDispatchers|AssignOnActorBeginOverlap _returnvalue_2 (delegate Custom|CustomEvent)))

(fn ConstructionScript)